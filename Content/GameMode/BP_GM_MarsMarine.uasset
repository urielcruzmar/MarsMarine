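; Game mode for a Mars marine shooter that runs endless, escalating waves of aliens, with music on start.
; Each wave multiplies the alien count and shortens the spawn interval by a difficulty multiplier.
; A looping timer spawns BP_Alien at random TargetPoints until the wave's count is used up.
; RegisterAlienDeath removes dead aliens from the tracked list and starts the next wave after a delay once all are gone.
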(event Custom|SpawnWave
  (CallFunction|SpawnAlien))

(event Custom|EndWave
  (Utilities|FlowControl|Delay 5.0)
  (CallFunction|StartNewWave))

(event EventBeginPlay
  (Audio|SpawnSound2D "/Game/Sounds/Music/ShooterGame_Music_Cue.ShooterGame_Music_Cue" 1.0 1.0 0.0 0)
  (Utilities|FlowControl|Delay 2.0)
  (CallFunction|StartNewWave))

(fn ConstructionScript)

(fn StartNewWave
  (Math|Integer|IncrementInt (Variables|Default|GetCurentWave)
    (:%20%20
      (CallFunction|IncreaseWaveDifficulty)
      (Utilities|Time|SetTimerbyFunctionName 0 "SpawnWave" (Variables|Default|GetSpawnTime) true))))

(fn GetRandomSpawnPoint
  (bind _outactors (Actor|GetAllActorsOfClass "/Script/Engine.TargetPoint"))
  (return (Utilities|Array|Get(acopy) _outactors (Math|Random|RandomIntegerinRange 0 (Utilities|Array|LastIndex _outactors)))))

(fn SpawnAlien
  (bind _output (CallFunction|GetRandomSpawnPoint))
  (Utilities|IsValid _output
    (:Is%20Valid
      (bind _returnvalue (Game|SpawnActorfromClass "/Game/Blueprints/Pawns/BP_Alien.BP_Alien_C" (Transformation|GetActorTransform _output) "AdjustIfPossibleButAlwaysSpawn" "MultiplyWithRoot" 0 0))
      (Utilities|IsValid _returnvalue
        (:Is%20Valid
          (Utilities|Array|Add (Variables|Default|GetAliens) _returnvalue)
          (bind _result (Math|Integer|DecrementInt (Variables|Default|GetAlienSpawnsRemaining))
            (:%20%20
              (if (== _result 0)
                (Utilities|Time|ClearTimerbyFunctionName 0 "SpawnWave")))))))))

(fn RegisterAlienDeath
  (params (Alien :type BP%20Alien%20Object%20Reference%20%28by%20ref%29))
  (Utilities|Array|RemoveItem (Variables|Default|GetAliens) Alien)
  (if (CallFunction|IsWaveCompleted)
    (CallFunction|EndWave)))

(fn IsWaveCompleted
  (return (and (Utilities|Array|IsEmpty (Variables|Default|GetAliens)) (== (Variables|Default|GetAlienSpawnsRemaining) 0))))

(fn IncreaseWaveDifficulty
  (bind _output_get (Variables|Default|SetWaveDifficulty (Math|Float|Round (* (Variables|Default|GetWaveDifficulty) (Variables|Default|GetDifficultyMultiplier)))))
  (Variables|Default|SetAlienSpawnsRemaining _output_get)
  (Variables|Default|SetSpawnTime (/ (Variables|Default|GetSpawnTime) (Variables|Default|GetDifficultyMultiplier))))